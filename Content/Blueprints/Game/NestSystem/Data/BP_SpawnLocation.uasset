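; BP_SpawnLocation is a spawn point in the nest system, paired with a BP_FinishActor and color-coded to its ButtonActor.
; SpawnActorFinish creates the finish actor at a fixed offset along negative Y and links the two to each other.
; The construction script keeps the finish actor's X aligned with its own, leaving Y and Z free.
; On construction and BeginPlay, its Plane gets a material that ButtonActor creates from the button's color.
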(event EventBeginPlay
  (CallFunction|SetMaterialPlane (Variables|Default|GetPlane)))

(fn ConstructionScript
  (bind _actorfinish (Variables|TurtleMoveSystem|GetActorFinish))
  (bind _returnvalue (Transformation|GetActorLocation _actorfinish))
  (Transformation|SetActorLocation (Variables|TurtleMoveSystem|GetActorFinish) (Math|Vector|MakeVector (.x (Transformation|GetActorLocation)) (.y _returnvalue) (.z _returnvalue)) false false)
  (CallFunction|SetMaterialPlane (Variables|Default|GetPlane)))

(fn SpawnActorFinish
  (bind _returnvalue (Game|SpawnActorfromClass "/Game/Blueprints/Game/NestSystem/Data/BP_FinishActor.BP_FinishActor_C" (Math|Transform|MakeTransform (TurtleMoveSystem|LocationSpawnFinish) "0, 0, 0" "1,1,1") "Undefined" 0 0))
  (bind _output_get (Variables|TurtleMoveSystem|SetActorFinish _returnvalue))
  (bind _output_get_2 (LocalVariables|SetL_ActorFinish _output_get))
  (Variables|/Game/Blueprints/Game/NestSystem/Data/BP_FinishActor.BP_FinishActor_C|SetSpawnActor _output_get_2 self)
  (Transformation|SetActorLocation (Variables|TurtleMoveSystem|GetActorFinish) (TurtleMoveSystem|LocationSpawnFinish) false false))

(fn LocationSpawnFinish
  (bind _returnvalue (Transformation|GetActorLocation))
  (bind (_x _y _z) (Math|Vector|BreakVector _returnvalue))
  (return (Math|Vector|MakeVector _x (- _y 1.5e+02) _z)))

(fn SetMaterialPlane
  (params (Actor%20In :type Primitive%20Component%20Object%20Reference))
  (bind _buttonactor (Variables|Info|GetButtonActor))
  (bind _output_get (Variables|Default|SetColor (Variables|/Game/Blueprints/Game/NestSystem/Data/BP_ButtonDefault.BP_ButtonDefault_C|GetColor _buttonactor)))
  (Default|CreateMaterial _buttonactor Actor%20In _output_get))