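; BP_ButtonDefault is a numbered, colored trigger button in the nest system that spawns a turtle when the player steps into its box.
; The first valid overlap spawns a MoveToSystem turtle with its default controller at the linked spawn actor, provided that actor has a finish actor.
; The construction script applies color through a dynamic material and sets the number text.
; CreateSpawnActor places a BP_SpawnLocation beside the button and links both.
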(event OnComponentBeginOverlap(Box)
  (params (OverlappedComponent :type Primitive%20Component%20Object%20Reference) (OtherActor :type Actor%20Object%20Reference) (OtherComp :type Primitive%20Component%20Object%20Reference) (OtherBodyIndex :type Integer) (bFromSweep :type Boolean) (SweepResult :type Hit%20Result%20Structure%20%28by%20ref%29))
  (Utilities|Casting|CastToBP_Player OtherActor)
  (Utilities|IsValid (Variables|TurtleMoveSystem|GetSpawnActor)
    (:Is%20Valid
      (Utilities|IsValid (Variables|/Game/Blueprints/Game/NestSystem/Data/BP_SpawnLocation.BP_SpawnLocation_C|GetActorFinish (Variables|TurtleMoveSystem|GetSpawnActor))
        (:Is%20Valid
          (if (not (Variables|Info|GetSpawn?))
            (CallFunction|SpawnTurtle)
            (Variables|Info|SetSpawn? true)))
        (:Is%20Not%20Valid
          (Development|PrintString "Please the create actor-finish"))))
    (:Is%20Not%20Valid
      (Development|PrintString "Please the create actor-spawn"))))

(event Custom|SpawnTurtle
  (Utilities|IsValid (Variables|TurtleMoveSystem|GetSpawnActor)
    (:Is%20Valid
      (bind _returnvalue (Game|SpawnActorfromClass "/Game/Blueprints/Game/NestSystem/BP_CharacterTurtleDefault.BP_CharacterTurtleDefault_C" (Math|Transform|MakeTransform (Transformation|GetActorLocation (Variables|TurtleMoveSystem|GetSpawnActor)) "0, 0, 0" "1,1,1") "Undefined" 0 (Variables|TurtleMoveSystem|GetMoveToSystem) 0))
      (bind _output_get (Variables|Info|SetCharacterTurtle _returnvalue))
      (Pawn|SpawnDefaultController _output_get))))

(event EventBeginPlay)

(fn ConstructionScript
  (TurtleMoveSystem|CreateMaterial (Variables|Default|GetCube) (Variables|TurtleMoveSystem|GetColor))
  (Rendering|Components|TextRender|SetText (Variables|Default|GetTextRender) (Utilities|Text|ToText(Integer) (Variables|TurtleMoveSystem|GetNumber))))

(fn CreateMaterial
  (params (Actor%20In :type Primitive%20Component%20Object%20Reference) (Value :type Linear%20Color%20Structure))
  (Variables|TurtleMoveSystem|SetColor Value)
  (bind _returnvalue (Rendering|Material|CreateDynamicMaterialInstance Actor%20In 0 "/Game/Assets/Materials/MI_Color4.MI_Color4" "None" :!class /Script/Engine.PrimitiveComponent))
  (Rendering|Material|SetVectorParameterValue _returnvalue "Color" (Variables|TurtleMoveSystem|GetColor) :!class /Script/Engine.MaterialInstanceDynamic)
  (return))

(fn CreateSpawnActor
  (bind _returnvalue (Transformation|GetActorLocation))
  (bind (_x _y _z) (Math|Vector|BreakVector _returnvalue))
  (Utilities|IsValid (Variables|TurtleMoveSystem|GetSpawnActor)
    (:Is%20Valid
      (Development|PrintString "Already created. Delete previous object 
" true true "(R=0.000000,G=0.660000,B=1.000000,A=1.000000)" 6.0))
    (:Is%20Not%20Valid
      (Development|PrintString "Creating spawn actor" true true "(R=0.000000,G=0.660000,B=1.000000,A=1.000000)" 6.0)
      (bind _returnvalue_2 (Game|SpawnActorfromClass "/Game/Blueprints/Game/NestSystem/Data/BP_SpawnLocation.BP_SpawnLocation_C" (Math|Transform|MakeTransform (Math|Vector|MakeVector _x (+ _y 1.5e+02) _z) "0, 0, 0" "1,1,1") "Undefined" 0 0))
      (bind _output_get (Variables|TurtleMoveSystem|SetSpawnActor _returnvalue_2))
      (Variables|/Game/Blueprints/Game/NestSystem/Data/BP_SpawnLocation.BP_SpawnLocation_C|SetButtonActor _output_get self))))