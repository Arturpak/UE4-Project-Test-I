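; BP_FinishActor is the finish trigger that marks the end of the course for the turtle character.
; When a BP_CharacterTurtleDefault overlaps its Box, it sets that character's Finish flag, reveals the Text component and fades in SCFinish.
; At construction, it snaps its X position to the referenced SpawnActor, keeping its own Y and Z, and has that actor set the plane material on its Cube.
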(event OnComponentBeginOverlap(Box)
  (params (OverlappedComponent :type Primitive%20Component%20Object%20Reference) (OtherActor :type Actor%20Object%20Reference) (OtherComp :type Primitive%20Component%20Object%20Reference) (OtherBodyIndex :type Integer) (bFromSweep :type Boolean) (SweepResult :type Hit%20Result%20Structure%20%28by%20ref%29))
  (bind _asbp_character_turtle_default (Utilities|Casting|CastToBP_CharacterTurtleDefault OtherActor))
  (Variables|/Game/Blueprints/Game/NestSystem/BP_CharacterTurtleDefault.BP_CharacterTurtleDefault_C|SetFinish? _asbp_character_turtle_default true)
  (Development|SetHiddeninGame (Variables|Default|GetText) false false)
  (Audio|Components|Audio|FadeIn (Variables|Default|GetSC_Finish) 1.0 1.0 0.0 "Linear" :!class /Script/Engine.AudioComponent))

(fn ConstructionScript
  (CallFunction|SetLocationSelf)
  (Default|SetMaterialPlane (Variables|TurtleMoveSystem|GetSpawnActor) (Variables|Default|GetCube)))

(fn SetLocationSelf
  (bind _returnvalue (Transformation|GetActorLocation))
  (Transformation|SetActorLocation self (Math|Vector|MakeVector (.x (Transformation|GetActorLocation (Variables|TurtleMoveSystem|GetSpawnActor))) (.y _returnvalue) (.z _returnvalue)) false false))