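; Default turtle character for the nest system that emerges with particles and sound, then travels until its Finish flag is set.
; BeginPlay applies a colored dynamic material, reveals the mesh after a delay, then picks a movement pattern from ETurtleMoveSystem: continuous, stop-and-go, or forward/back.
; Looping timers drive AddMovementInput, with delay loops alternating the phases and PlaySound fading movement audio.
; The forward/back pattern's second phase uses a fixed +Y direction instead of WorldDirection.
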(event Custom|PlaySound
  (params (Condition :type Boolean))
  (bind _movementturtle (Variables|Default|GetMovementTurtle))
  (if (Variables|Default|GetFinish?)
    (Audio|Components|Audio|FadeOut (Variables|Default|GetMovementTurtle) 0.4 0.0 "Linear" :!class /Script/Engine.AudioComponent)
    (elif Condition
      (Audio|Components|Audio|FadeIn _movementturtle 1.0 1.0 0.0 "Linear" :!class /Script/Engine.AudioComponent)
      (else
        (Audio|Components|Audio|FadeOut _movementturtle 0.28 0.5 "Linear" :!class /Script/Engine.AudioComponent)))))

(event EventBeginPlay
  (CallFunction|CreateMaterialInstance)
  (CallFunction|FunctionParticleEmergence true)
  (Audio|Components|Audio|FadeIn (Variables|Default|GetSoundSpawn) 0.3 0.3 0.0 "Linear" :!class /Script/Engine.AudioComponent)
  (Utilities|FlowControl|Delay 3.0)
  (CallFunction|FunctionParticleEmergence false)
  (Development|SetHiddeninGame (Variables|Default|GetStaticMesh) false false)
  (switch Utilities|FlowControl|Switch|SwitchonE_TurtleMoveSystem (Variables|TurtleMoveSystem|GetE_TurtleMoveSystem)
    (:NewEnumerator0
      (bind _returnvalue (Utilities|Time|SetTimerbyFunctionName 0 "FunctionMoveTo" 0.01 true))
      (Variables|Default|SetTimer _returnvalue)
      (CallFunction|PlaySound true)
      (if (Variables|Default|GetFinish?)
        (Utilities|Time|ClearandInvalidateTimerbyHandle (Variables|Default|GetTimer))))
    (:NewEnumerator1
      (bind _returnvalue_2 (Utilities|Time|SetTimerbyFunctionName 0 "FunctionMoveTo" 0.01 true :!label _label))
      (Variables|Default|SetTimer _returnvalue_2)
      (CallFunction|PlaySound true)
      (Utilities|FlowControl|Delay 1.0)
      (Utilities|Time|ClearandInvalidateTimerbyHandle (Variables|Default|GetTimer))
      (CallFunction|PlaySound false)
      (Utilities|FlowControl|Delay 0.5)
      (if (Variables|Default|GetFinish?)
        (Utilities|Time|ClearandInvalidateTimerbyHandle (Variables|Default|GetTimer))
        (else
          (goto _label))))
    (:NewEnumerator2
      (bind _returnvalue_3 (Utilities|Time|SetTimerbyFunctionName 0 "FunctionMoveTo" 0.01 true :!label _label_2))
      (Variables|Default|SetTimer _returnvalue_3)
      (CallFunction|PlaySound true)
      (Utilities|FlowControl|Delay 1.0)
      (Utilities|Time|ClearandInvalidateTimerbyHandle (Variables|Default|GetTimer))
      (CallFunction|PlaySound true)
      (bind _returnvalue_4 (Utilities|Time|SetTimerbyFunctionName 0 "FunctionMoveToF_B" 0.01 true))
      (Variables|Default|SetTimer _returnvalue_4)
      (Utilities|FlowControl|Delay 0.5)
      (Utilities|Time|ClearandInvalidateTimerbyHandle (Variables|Default|GetTimer))
      (if (Variables|Default|GetFinish?)
        (Utilities|Time|ClearandInvalidateTimerbyHandle (Variables|Default|GetTimer))
        (else
          (goto _label_2))))))

(fn ConstructionScript)

(fn FunctionMoveto
  (if (Variables|Default|GetFinish?)
    (Utilities|Time|ClearandInvalidateTimerbyHandle (Variables|Default|GetTimer))
    (CallFunction|PlaySound false)
    (else
      (Pawn|Input|AddMovementInput self (Variables|Default|GetWorld%20Direction) 0.8 true))))

(fn FunctionMovetoFB
  (if (Variables|Default|GetFinish?)
    (Utilities|Time|ClearandInvalidateTimerbyHandle (Variables|Default|GetTimer))
    (else
      (Pawn|Input|AddMovementInput self "0.000000,1.000000, 0" 1.0 true))))

(fn FunctionParticleEmergence
  (params (Activate? :type Boolean))
  (bind _particle (Variables|Default|GetParticle))
  (if Activate?
    (Components|Activation|Activate _particle false)
    (else
      (Components|Activation|Deactivate _particle))))

(fn CreateMaterialInstance
  (bind _returnvalue (Rendering|Material|CreateDynamicMaterialInstance "/Game/Assets/Materials/MI_Color4.MI_Color4" "None" "None" :!class /Script/Engine.KismetMaterialLibrary))
  (bind _output_get (Variables|Default|SetMaterialInstance _returnvalue))
  (Rendering|Material|SetMaterial (Variables|Default|GetStaticMesh) 0 _output_get)
  (Rendering|Material|SetVectorParameterValue (Variables|Default|GetMaterialInstance) "Color" (Variables|Default|GetColorCube) :!class /Script/Engine.MaterialInstanceDynamic))