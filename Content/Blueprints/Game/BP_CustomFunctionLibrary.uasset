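; BP_CustomFunctionLibrary is a set of helper functions that give quick typed access to core player objects.
; It returns player index 0's HUD, character and controller, cast to BP_HUD, BP_Player and BP_PlayerContoller.
; Each function returns a value only when its cast succeeds, with no handling for failure.
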(fn HUDController
  (bind _asbp_hud (Utilities|Casting|CastToBP_HUD (HUD|GetHUD (Game|GetPlayerController 0))))
  (return _asbp_hud))

(fn PlayerCharacter
  (bind _asbp_player (Utilities|Casting|CastToBP_Player (Game|GetPlayerCharacter 0)))
  (return _asbp_player))

(fn PlayerContoller
  (bind _asbp_player_contoller (Utilities|Casting|CastToBP_PlayerContoller (Game|GetPlayerController 0)))
  (return _asbp_player_contoller))